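; Portal actor paired with LinkedPortal that shows a live view through its twin and teleports overlapping actors that cross its plane.
; Each tick the linked scene capture, placed by mirroring the player camera, renders recursively up to MaxRecursion into a viewport-sized render target on the portal material.
; Crossing uses a front-to-back sign change plus line-plane intersection.
; Teleporting mirrors the actor's transform, but always adjusts the player's control rotation and velocity.
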(event `self.ReceiveBeginPlay`
  (bind (_returnvalue_x _returnvalue_y) (`KismetMathLibrary.BreakVector2D` (`WidgetLayoutLibrary.GetViewportSize`)))
  (bind (_returnvalue_x_2 _returnvalue_y_2 _returnvalue_z) (`KismetMathLibrary.BreakVector` (* (`SceneComponent.GetForwardVector` (`self.ForwardDirection`)) (`self.OffsetAmount`))))
  (`KismetSystemLibrary.Delay` 0.01)
  (`/Engine/EditorBlueprintResources/StandardMacros.IsValid` (`self.LinkedPortal`)
    (:`Is Valid`
      (`self.SetTickGroup` "TG_PostUpdateWork")
      (bind _returnvalue (`KismetMaterialLibrary.CreateDynamicMaterialInstance` "/Game/PortalSystem/M_Portal.M_Portal"))
      (bind _output_get (set `self.M_Portal` _returnvalue))
      (`PrimitiveComponent.SetMaterial` (`self.PortalPlane`) 0 _output_get)
      (bind _returnvalue_2 (`KismetRenderingLibrary.CreateRenderTarget2D` (`KismetMathLibrary.FTrunc` _returnvalue_x) (`KismetMathLibrary.FTrunc` _returnvalue_y)))
      (bind _output_get_2 (set `self.Portal_RT` _returnvalue_2))
      (`MaterialInstanceDynamic.SetTextureParameterValue` (`self.M_Portal`) "Texture" _output_get_2)
      (set `SceneCaptureComponent2D.TextureTarget` (`self.Portal_RT`) (`/Game/PortalSystem/Portal_BP.PortalCamera` (`self.LinkedPortal`)))
      (`self.SetClipPlane`)
      (`MaterialInstanceDynamic.SetVectorParameterValue` (`self.M_Portal`) "OffsetDistance" (`KismetMathLibrary.MakeColor` _returnvalue_x_2 _returnvalue_y_2 _returnvalue_z))
      (bind _asbp_first_person_character (cast `/Game/FirstPerson/Blueprints/BP_FirstPersonCharacter` (`GameplayStatics.GetPlayerCharacter` 0))
        (:`then`
          (`/Engine/EditorBlueprintResources/StandardMacros.IsValid` (`/Game/FirstPerson/Blueprints/BP_FirstPersonCharacter.Portal1` _asbp_first_person_character)
            (:`Is Valid`
              (`/Engine/EditorBlueprintResources/StandardMacros.IsValid` (`/Game/FirstPerson/Blueprints/BP_FirstPersonCharacter.Portal2` _asbp_first_person_character)
                (:`Is Valid`
                  (`KismetSystemLibrary.PrintString` "failrfffff"))
                (:`Is Not Valid`
                  (set `/Game/FirstPerson/Blueprints/BP_FirstPersonCharacter.Portal2` self _asbp_first_person_character))))
            (:`Is Not Valid`
              (set `/Game/FirstPerson/Blueprints/BP_FirstPersonCharacter.Portal1` self _asbp_first_person_character))))
        (:`CastFailed`
          (`KismetSystemLibrary.PrintString` "failed"))))))

(event `self.ReceiveTick`
  (params (DeltaSeconds :type "Float (single-precision)"))
  (`/Engine/EditorBlueprintResources/StandardMacros.IsValid` (`self.LinkedPortal`)
    (:`Is Valid`
      (`self.UpdateSceneCaptureRecursive` (0.0 0.0 0.0))
      (`self.CheckViewportSize`)
      (`self.ShouldTeleport`))))

(fn `CheckViewportSize`
  (bind (_returnvalue_x _returnvalue_y) (`KismetMathLibrary.BreakVector2D` (`WidgetLayoutLibrary.GetViewportSize`)))
  (bind _portal_rt (`self.Portal_RT`))
  (bind (_x _y) (`KismetMathLibrary.BreakVector2D` (`WidgetLayoutLibrary.GetViewportSize`)))
  (`/Engine/EditorBlueprintResources/StandardMacros.IsValid` (`self.Portal_RT`)
    (:`Is Valid`
      (if (not (and (== _x (`TextureRenderTarget2D.SizeX` _portal_rt)) (== _y (`TextureRenderTarget2D.SizeY` _portal_rt))))
        (`KismetRenderingLibrary.ResizeRenderTarget2D` (`self.Portal_RT`) (`KismetMathLibrary.FTrunc` _returnvalue_x) (`KismetMathLibrary.FTrunc` _returnvalue_y))))))

(fn `IsPointCrossingPortal`
  (params (Point :type "Vector Structure") (PortalLocation :type "Vector Structure") (PortalNormal :type "Vector Structure"))
  (returns (return :type Boolean))
  (locals (IsInFront :type Boolean) (PortalPlane :type "Plane Structure") (IsIntersect :type Boolean :default false) (IsCrossing :type Boolean :default false))
  (set `local.IsInFront` (>= (`KismetMathLibrary.Dot_VectorVector` PortalNormal (- Point PortalLocation)) 0.0))
  (bind _output_get (set `local.PortalPlane` (`KismetMathLibrary.MakePlaneFromPointAndNormal` (`local.PortalLocation`) (`local.PortalNormal`))))
  (set `local.IsIntersect` (`.ReturnValue` (`KismetMathLibrary.LinePlaneIntersection` (`self.LastPosition`) (`local.Point`) _output_get)))
  (set `local.IsCrossing` (and (`local.IsIntersect`) (not (`local.IsInFront`)) (`self.LastInFront`)))
  (set `self.LastInFront` (`local.IsInFront`))
  (set `self.LastPosition` (`local.Point`))
  (return (`local.IsCrossing`)))

(fn `SetClipPlane`
  (bind _portalcamera (`self.PortalCamera`))
  (`/Engine/EditorBlueprintResources/StandardMacros.IsValid` (`self.LinkedPortal`)
    (:`Is Valid`
      (set `SceneCaptureComponent2D.bEnableClipPlane` true _portalcamera)
      (set `SceneCaptureComponent2D.ClipPlaneBase` (+ (`SceneComponent.K2_GetComponentLocation` (`self.PortalPlane`)) (* (`SceneComponent.GetForwardVector` (`self.ForwardDirection`)) (0.0 0.0 0.0))) _portalcamera)
      (set `SceneCaptureComponent2D.ClipPlaneNormal` (`SceneComponent.GetForwardVector` (`self.ForwardDirection`)) _portalcamera))))

(fn `SetLocation`
  (params (Location :type "Vector Structure"))
  (returns (ReturnValue :type "Vector Structure"))
  (return (`KismetMathLibrary.TransformLocation` (`self.GetTransform` (`self.LinkedPortal`)) (`KismetMathLibrary.InverseTransformLocation` (`KismetMathLibrary.MakeTransform` (.location (`self.GetTransform`)) (.rotation (`self.GetTransform`)) (`KismetMathLibrary.MakeVector` (* (.x (.scale (`self.GetTransform`))) -1.0) (* (.y (.scale (`self.GetTransform`))) -1.0) (.z (.scale (`self.GetTransform`))))) Location))))

(fn `SetRotation`
  (params (InRot :type "Rotator Structure (by ref)"))
  (returns (ReturnValue :type "Rotator Structure"))
  (bind (_x _y _z) (`KismetMathLibrary.BreakRotIntoAxes` InRot))
  (bind _returnvalue (`self.GetTransform`))
  (bind _returnvalue_2 (`self.GetTransform` (`self.LinkedPortal`)))
  (return (`KismetMathLibrary.MakeRotationFromAxes` (`KismetMathLibrary.TransformDirection` _returnvalue_2 (`KismetMathLibrary.MirrorVectorByNormal` (`KismetMathLibrary.MirrorVectorByNormal` (`KismetMathLibrary.InverseTransformDirection` _returnvalue _x) (1.0 0.0 0.0)) (0.0 1.0 0.0))) (`KismetMathLibrary.TransformDirection` _returnvalue_2 (`KismetMathLibrary.MirrorVectorByNormal` (`KismetMathLibrary.MirrorVectorByNormal` (`KismetMathLibrary.InverseTransformDirection` _returnvalue _y) (1.0 0.0 0.0)) (0.0 1.0 0.0))) (`KismetMathLibrary.TransformDirection` _returnvalue_2 (`KismetMathLibrary.MirrorVectorByNormal` (`KismetMathLibrary.MirrorVectorByNormal` (`KismetMathLibrary.InverseTransformDirection` _returnvalue _z) (1.0 0.0 0.0)) (0.0 1.0 0.0))))))

(fn `ShouldTeleport`
  (bind _overlappingactors (`PrimitiveComponent.GetOverlappingActors` (`self.PlayerDetection`) "/Script/Engine.Actor"))
  (if (> (`KismetArrayLibrary.Array_Length` _overlappingactors) 0)
    (for _array_element _overlappingactors
      (`/Engine/EditorBlueprintResources/StandardMacros.IsValid` _array_element
        (:`Is Valid`
          (bind _output_get (set `self.Actor to tp` _array_element))
          (bind _asbp_first_person_character (cast `/Game/FirstPerson/Blueprints/BP_FirstPersonCharacter` _output_get)
            (:`then`
              (bind _return (`self.IsPointCrossingPortal` (`SceneComponent.K2_GetComponentLocation` (`PortalCharacter.FirstPersonCameraComponent` _asbp_first_person_character)) (`self.K2_GetActorLocation`) (`SceneComponent.GetForwardVector` (`self.ForwardDirection`)))))
            (:`CastFailed`
              (bind _return_2 (`self.IsPointCrossingPortal` (`SceneComponent.K2_GetComponentLocation` (`Actor.RootComponent` (`self.Actor to tp`))) (`self.K2_GetActorLocation`) (`SceneComponent.GetForwardVector` (`self.ForwardDirection`))))))
          (if (or _return _return_2)
            (`self.TeleportCharacter`)))))))

(fn `TeleportCharacter`
  (bind _returnvalue (`self.UpdateControlRotation`))
  (bind _returnvalue_2 (`Pawn.GetMovementComponent` (`GameplayStatics.GetPlayerCharacter` 0)))
  (`self.K2_SetActorTransform` (`self.Actor to tp`) (`KismetMathLibrary.MakeTransform` (`self.UpdateLocation`) (`self.UpdateRotation`)) false false)
  (`Controller.SetControlRotation` (`GameplayStatics.GetPlayerController` 0) _returnvalue)
  (bind _returnvalue_3 (`self.UpdateVelocity` (`MovementComponent.Velocity` _returnvalue_2)))
  (set `MovementComponent.Velocity` _returnvalue_3 _returnvalue_2)
  (`/Game/FirstPerson/Blueprints/BP_FirstPersonCharacter.SmoothOrientation` (cast `/Game/FirstPerson/Blueprints/BP_FirstPersonCharacter` (`GameplayStatics.GetPlayerCharacter` 0) :!pure true) _returnvalue)
  (`PlayerCameraManager.SetGameCameraCutThisFrame` (`GameplayStatics.GetPlayerCameraManager` 0)))

(fn `UpdateControlRotation`
  (returns (ReturnValue :type "Rotator Structure"))
  (bind _returnvalue (`self.GetTransform`))
  (bind (_x _y _z) (`KismetMathLibrary.GetAxes` (`self.K2_GetActorRotation` (`GameplayStatics.GetPlayerController` 0))))
  (return (`KismetMathLibrary.MakeRotationFromAxes` (`KismetMathLibrary.TransformDirection` (`self.GetTransform` (`self.LinkedPortal`)) (`KismetMathLibrary.MirrorVectorByNormal` (`KismetMathLibrary.MirrorVectorByNormal` (`KismetMathLibrary.InverseTransformDirection` _returnvalue _x) (1.0 0.0 0.0)) (0.0 1.0 0.0))) (`KismetMathLibrary.TransformDirection` (`self.GetTransform` (`self.LinkedPortal`)) (`KismetMathLibrary.MirrorVectorByNormal` (`KismetMathLibrary.MirrorVectorByNormal` (`KismetMathLibrary.InverseTransformDirection` _returnvalue _y) (1.0 0.0 0.0)) (0.0 1.0 0.0))) (`KismetMathLibrary.TransformDirection` (`self.GetTransform` (`self.LinkedPortal`)) (`KismetMathLibrary.MirrorVectorByNormal` (`KismetMathLibrary.MirrorVectorByNormal` (`KismetMathLibrary.InverseTransformDirection` _returnvalue _z) (1.0 0.0 0.0)) (0.0 1.0 0.0))))))

(fn `UpdateLocation`
  (returns (ReturnValue :type "Vector Structure"))
  (bind _returnvalue (`self.GetTransform`))
  (return (`KismetMathLibrary.TransformLocation` (`self.GetTransform` (`self.LinkedPortal`)) (`KismetMathLibrary.InverseTransformLocation` (`KismetMathLibrary.MakeTransform` (.location _returnvalue) (.rotation _returnvalue) (`KismetMathLibrary.MakeVector` (* (.x (.scale _returnvalue)) -1.0) (* (.y (.scale _returnvalue)) -1.0) (.z (.scale _returnvalue)))) (`self.K2_GetActorLocation` (`self.Actor to tp`))))))

(fn `UpdateRotation`
  (returns (ReturnValue :type "Rotator Structure"))
  (bind _returnvalue (`self.GetTransform`))
  (bind (_x _y _z) (`KismetMathLibrary.GetAxes` (`self.K2_GetActorRotation` (`self.Actor to tp`))))
  (return (`KismetMathLibrary.MakeRotationFromAxes` (`KismetMathLibrary.TransformDirection` (`self.GetTransform` (`self.LinkedPortal`)) (`KismetMathLibrary.MirrorVectorByNormal` (`KismetMathLibrary.MirrorVectorByNormal` (`KismetMathLibrary.InverseTransformDirection` _returnvalue _x) (1.0 0.0 0.0)) (0.0 1.0 0.0))) (`KismetMathLibrary.TransformDirection` (`self.GetTransform` (`self.LinkedPortal`)) (`KismetMathLibrary.MirrorVectorByNormal` (`KismetMathLibrary.MirrorVectorByNormal` (`KismetMathLibrary.InverseTransformDirection` _returnvalue _y) (1.0 0.0 0.0)) (0.0 1.0 0.0))) (`KismetMathLibrary.TransformDirection` (`self.GetTransform` (`self.LinkedPortal`)) (`KismetMathLibrary.MirrorVectorByNormal` (`KismetMathLibrary.MirrorVectorByNormal` (`KismetMathLibrary.InverseTransformDirection` _returnvalue _z) (1.0 0.0 0.0)) (0.0 1.0 0.0))))))

(fn `UpdateSceneCapture`
  (`SceneComponent.K2_SetWorldLocationAndRotation` :`self` (`/Game/PortalSystem/Portal_BP.PortalCamera` (`self.LinkedPortal`))))

(fn `UpdateSceneCaptureRecursive`
  (params (Location :type "Vector Structure") (Rotation :type "Rotator Structure"))
  (locals (TemporaryLocation :type "Vector Structure") (TemporaryRotation :type "Rotator Structure"))
  (bind _transformcomponent (`PlayerCameraManager.TransformComponent` (`GameplayStatics.GetPlayerCameraManager` 0)))
  (if (== (`self.CurrentRecursion`) 0)
    (set `local.TemporaryLocation` (`self.SetLocation` (`SceneComponent.K2_GetComponentLocation` _transformcomponent)))
    (set `local.TemporaryRotation` (`self.SetRotation` (`SceneComponent.K2_GetComponentRotation` _transformcomponent)))
    (`/Engine/EditorBlueprintResources/StandardMacros.IncrementInt` (`self.CurrentRecursion`)
      (:`  `
        (`self.UpdateSceneCaptureRecursive` (`local.TemporaryLocation`) (`local.TemporaryRotation`))
        (`SceneComponent.K2_SetWorldLocationAndRotation` (`/Game/PortalSystem/Portal_BP.PortalCamera` (`self.LinkedPortal`)) (`local.TemporaryLocation`) (`local.TemporaryRotation`) false false)
        (`SceneCaptureComponent2D.CaptureScene` (`/Game/PortalSystem/Portal_BP.PortalCamera` (`self.LinkedPortal`)))
        (set `self.CurrentRecursion` 0)))
    (elif (< (`self.CurrentRecursion`) (`self.MaxRecursion`))
      (set `local.TemporaryLocation` (`self.SetLocation` (`local.Location`)))
      (set `local.TemporaryRotation` (`self.SetRotation` (`local.Rotation`)))
      (`/Engine/EditorBlueprintResources/StandardMacros.IncrementInt` (`self.CurrentRecursion`)
        (:`  `
          (`self.UpdateSceneCaptureRecursive` (`local.TemporaryLocation`) (`local.TemporaryRotation`))
          (`SceneComponent.K2_SetWorldLocationAndRotation` (`/Game/PortalSystem/Portal_BP.PortalCamera` (`self.LinkedPortal`)) (`local.TemporaryLocation`) (`local.TemporaryRotation`) false false)
          (`SceneCaptureComponent2D.CaptureScene` (`/Game/PortalSystem/Portal_BP.PortalCamera` (`self.LinkedPortal`)))))
      (else
        (`SceneComponent.K2_SetWorldLocationAndRotation` (`/Game/PortalSystem/Portal_BP.PortalCamera` (`self.LinkedPortal`)) (`self.SetLocation` (`local.Location`)) (`self.SetRotation` (`local.Rotation`)) false false)
        (`SceneComponent.SetVisibility` (`self.PortalPlane`) false false)
        (`SceneCaptureComponent2D.CaptureScene` (`/Game/PortalSystem/Portal_BP.PortalCamera` (`self.LinkedPortal`)))
        (`SceneComponent.SetVisibility` (`self.PortalPlane`) true false)))))

(fn `UpdateVelocity`
  (params (Velocity :type "Vector Structure"))
  (returns (ReturnValue :type "Vector Structure"))
  (return (* (`KismetMathLibrary.TransformDirection` (`self.GetTransform` (`self.LinkedPortal`)) (`KismetMathLibrary.MirrorVectorByNormal` (`KismetMathLibrary.MirrorVectorByNormal` (`KismetMathLibrary.InverseTransformDirection` (`self.GetTransform`) (`KismetMathLibrary.Normal` Velocity)) (1.0 0.0 0.0)) (0.0 1.0 0.0))) (`KismetMathLibrary.VSize` (`local.Velocity`)))))

(fn `UserConstructionScript`)